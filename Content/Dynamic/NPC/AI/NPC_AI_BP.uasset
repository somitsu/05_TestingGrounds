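; NPC AI controller for patrolling guards, running the BT_GuardBehaviour tree on the BB_PatrolData blackboard.
; AI Perception writes sensed actors without the "Enemy" tag to the blackboard's enemy key and clears it when such an actor is lost.
; Every tick, the controlled BP_PatrollingGuard2 has its Aiming and Shooting flags set by whether the controller has a valid focus actor.
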(event `self.ReceiveBeginPlay`
  (bind _blackboardcomponent (`self.UseBlackboard` "/Game/Dynamic/NPC/AI/BB_PatrolData.BB_PatrolData"))
  (`self.RunBehaviorTree` "/Game/Dynamic/NPC/AI/BT_GuardBehaviour.BT_GuardBehaviour")
  (set `self.blackBoardComp` _blackboardcomponent))

(event `self.ReceiveTick`
  (params (DeltaSeconds :type "Float (single-precision)"))
  (bind _returnvalue (`KismetSystemLibrary.IsValid` (`self.GetFocusActor`)))
  (bind _asbp_patrolling_guard_2 (cast `/Game/Dynamic/NPC/Behaviour/BP_PatrollingGuard2` (`self.K2_GetPawn`)))
  (set `/Game/Dynamic/NPC/Behaviour/BP_PatrollingGuard2.Aiming` _returnvalue _asbp_patrolling_guard_2)
  (set `/Game/Dynamic/NPC/Behaviour/BP_PatrollingGuard2.Shooting` _returnvalue _asbp_patrolling_guard_2))

(event `self.AIPerception.OnTargetPerceptionUpdated`
  (params (Actor :type "Actor Object Reference") (Stimulus :type "AIStimulus Structure"))
  (bind _enemykey (`self.enemyKey`))
  (bind _blackboardcomp (`self.blackBoardComp`))
  (if (`self.ActorHasTag` Actor "Enemy")
    _
    (elif (`.bSuccessfullySensed` (break `AIStimulus` Stimulus))
      (`BlackboardComponent.SetValueAsObject` _blackboardcomp _enemykey Actor)
      (else
        (`BlackboardComponent.ClearValue` _blackboardcomp _enemykey)))))

(fn `UserConstructionScript`)