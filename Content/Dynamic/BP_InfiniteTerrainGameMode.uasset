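; Game mode for an infinite terrain game that spawns the starting run of tiles and keeps the score.
; On BeginPlay it fills a nav mesh bounds volume pool, then calls SpawnTiles several times.
; Each new BP_Tile receives the shared pool, and its attach location becomes the next spawn transform, chaining tiles end to end.
; NewTileConquered increments the score, which GetScore exposes.
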(event `self.ReceiveBeginPlay`
  (`self.populateBoundsVolumePool`)
  (for _ (range 4)
    (`self.SpawnTiles`)))

(fn `getScore`
  (returns (score :type Integer))
  (return (`self.score`)))

(fn `newTileConquered`
  (`/Engine/EditorBlueprintResources/StandardMacros.IncrementInt` (`self.score`)))

(fn `SpawnTiles`
  (bind _returnvalue (`|SpawnActorFromClass` "/Game/Dynamic/Terrain/BP_Tile.BP_Tile_C" (`self.nextTileTransform`) "Undefined" "OverrideRootScale" null null))
  (`Tile.setPool` _returnvalue (`self.navMeshBoundsVolumePool`))
  (bind _attachtransform (`/Game/Dynamic/Terrain/BP_Tile.GetAttachLocation` _returnvalue))
  (set `self.nextTileTransform` _attachtransform))

(fn `UserConstructionScript`)