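; BP_Tile is one segment of an infinite terrain, scattered at BeginPlay with random containers, props and rocks via PlaceActors.
; Its barrier starts locked (red, colliding) and unlocks (green, no collision) while the player is inside LockVolume.
; Leaving LockVolume relocks it and asks GM_InfiniteTerrain to spawn tiles, while entering DestroyVolume destroys the tile.
; GetAttachLocation exposes the Arrow's world transform as an attach point.
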(event `self.ReceiveBeginPlay`
  (`self.Lock`)
  (`self.PlaceActors` "/Game/Dynamic/Terrain/Props/BP_Container.BP_Container_C" 1 3)
  (`self.PlaceActors` "/Game/Dynamic/Terrain/Props/BP_Box.BP_Box_C" 2 4)
  (`self.PlaceActors` "/Game/Dynamic/Terrain/Props/BP_Canister.BP_Canister_C" 1 7)
  (`self.PlaceActors` "/Game/Dynamic/Terrain/Props/BP_Rock01_High.BP_Rock01_High_C" 0 4)
  (`self.PlaceActors` "/Game/Dynamic/Terrain/Props/BP_Rock05_High.BP_Rock05_High_C" 0 4)
  (`self.PlaceActors` "/Game/Dynamic/Terrain/Props/BP_Rock17_High.BP_Rock17_High_C" 0 4)
  (`self.PlaceActors` "/Game/Dynamic/Terrain/Props/BP_Rocks.BP_Rocks_C" 0 2)
  (`self.PlaceActors` "/Game/Dynamic/Terrain/Props/BP_Sandbags.BP_Sandbags_C" 0 2))

(event `self.LockVolume.OnComponentEndOverlap`
  (params (OverlappedComponent :type "PrimitiveComponent Object Reference") (OtherActor :type "Actor Object Reference") (OtherComp :type "PrimitiveComponent Object Reference") (OtherBodyIndex :type Integer))
  (`self.IsPlayerCharacter` OtherActor)
  (`self.Lock`)
  (bind _asgm_infinite_terrain (cast `/Game/Dynamic/GM_InfiniteTerrain` (`GameplayStatics.GetGameMode`)))
  (`/Game/Dynamic/GM_InfiniteTerrain.SpawnTiles` _asgm_infinite_terrain))

(event `self.LockVolume.OnComponentBeginOverlap`
  (params (OverlappedComponent :type "PrimitiveComponent Object Reference") (OtherActor :type "Actor Object Reference") (OtherComp :type "PrimitiveComponent Object Reference") (OtherBodyIndex :type Integer) (bFromSweep :type Boolean) (SweepResult :type "HitResult Structure (by ref)"))
  (`self.IsPlayerCharacter` OtherActor)
  (`self.Unlock`))

(event `self.DestroyVolume.OnComponentBeginOverlap`
  (params (OverlappedComponent :type "PrimitiveComponent Object Reference") (OtherActor :type "Actor Object Reference") (OtherComp :type "PrimitiveComponent Object Reference") (OtherBodyIndex :type Integer) (bFromSweep :type Boolean) (SweepResult :type "HitResult Structure (by ref)"))
  (`self.IsPlayerCharacter` OtherActor)
  (`self.K2_DestroyActor`))

(fn `GetAttachLocation`
  (returns (AttachTransform :type "Transform Structure"))
  (return (`SceneComponent.K2_GetComponentToWorld` (`self.Arrow`))))

(fn `Lock`
  (`PrimitiveComponent.SetCollisionEnabled` (`self.StaticMesh`) "QueryAndPhysics")
  (`PrimitiveComponent.SetMaterial` (`self.StaticMesh`) 0 "/Game/Dynamic/Terrain/MI_Barrier_Red.MI_Barrier_Red"))

(fn `Unlock`
  (`PrimitiveComponent.SetCollisionEnabled` (`self.StaticMesh`) "NoCollision")
  (`PrimitiveComponent.SetMaterial` (`self.StaticMesh`) 0 "/Game/Dynamic/Terrain/MI_Barrier_Green.MI_Barrier_Green"))

(fn `UserConstructionScript`)